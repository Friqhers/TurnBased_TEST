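; BP_Pawn is a pawn Blueprint that switches its player controller between game-only and game-and-UI input.
; BeginPlay starts in game-only mode, and the Y key calls ToggleInput, which flips the IsGameInputMode flag, input mode and mouse cursor visibility.
; Tick prints the control rotation yaw to the screen each frame.
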(event Custom|ToggleInput
  (bind _asplayer_controller (Utilities|Casting|CastToPlayerController (Pawn|GetController)))
  (if (Variables|Default|GetbIsGameInputMode)
    (Input|SetInputModeGameandUI _asplayer_controller 0 "DoNotLock" true false)
    (Variables|/Script/Engine.PlayerController|SetbShowMouseCursor _asplayer_controller true)
    (Variables|Default|SetbIsGameInputMode false)
    (else
      (Input|SetInputModeGameOnly _asplayer_controller false)
      (Variables|/Script/Engine.PlayerController|SetbShowMouseCursor _asplayer_controller false)
      (Variables|Default|SetbIsGameInputMode true))))

(event EventBeginPlay
  (bind _asplayer_controller (Utilities|Casting|CastToPlayerController (Pawn|GetController)))
  (Input|SetInputModeGameOnly _asplayer_controller false)
  (Variables|Default|SetbIsGameInputMode true))

(event Collision|EventActorBeginOverlap
  (params (OtherActor :type Actor%20Object%20Reference)))

(event EventTick
  (params (DeltaSeconds :type Float%20%28single-precision%29))
  (Development|PrintString (Utilities|String|ToString(Float) (.yaw (Pawn|GetControlRotation :!class /Script/Engine.Pawn))) true true "(R=0.000000,G=0.660000,B=1.000000,A=1.000000)" 0.0))

(event Input|KeyboardEvents|Y
  (params (Key :type Key%20Structure :default "None"))
  (:Pressed
    (CallFunction|ToggleInput)))

(fn ConstructionScript)