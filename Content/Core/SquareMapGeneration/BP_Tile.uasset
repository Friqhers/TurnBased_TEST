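; BP_Tile is a square-map tile actor whose floor color reflects the mammal occupying it.
; Its construction script creates a dynamic instance of M_Tile on the floor mesh, and BeginPlay caches that material's TileColor as the default.
; OnTileUpdated sets TileColor back to the default when the tile is empty, or to the referenced mammal's current tile color otherwise.
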(event EventBeginPlay
  (bind _returnvalue (Rendering|Material|GetVectorParameterValue (Variables|Default|GetTileMatIns) "TileColor" :!class /Script/Engine.MaterialInstanceDynamic))
  (Variables|Default|SetDefaultColor _returnvalue))

(event Collision|EventActorBeginOverlap
  (params (OtherActor :type Actor%20Object%20Reference)))

(event EventTick
  (params (DeltaSeconds :type Float%20%28single-precision%29)))

(event EventOnTileUpdated
  (if (Class|TBTile|IsTileEmpty)
    (Rendering|Material|SetVectorParameterValue (Variables|Default|GetTileMatIns) "TileColor" (Variables|Default|GetDefaultColor) :!class /Script/Engine.MaterialInstanceDynamic)
    (else
      (Rendering|Material|SetVectorParameterValue (Variables|Default|GetTileMatIns) "TileColor" (Variables|/Script/TurnBasedCatMouse.TBMammalBase|GetCurrentTileColor (Variables|Default|GetMammalRef)) :!class /Script/Engine.MaterialInstanceDynamic))))

(fn ConstructionScript
  (bind _returnvalue (Rendering|Material|CreateDynamicMaterialInstance (Variables|Default|GetTileFloorMesh) 0 "/Game/Core/Materials/M_Tile.M_Tile" "None" :!class /Script/Engine.PrimitiveComponent))
  (Variables|Default|SetTileMatIns _returnvalue))